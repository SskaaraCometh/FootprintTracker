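; BP_Capture is an actor that maintains a persistent render target from an orthographic scene capture, apparently for snow deformation trails.
; At BeginPlay it publishes the capture's ortho width to MPC_Capture, creates a dynamic M_DrawToPersistent material and clears RT_Capture and RT_Persistent to black.
; Each tick it draws that material into RT_Persistent, which is never cleared after startup.
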(event `self.ReceiveBeginPlay`
  (`KismetMaterialLibrary.SetScalarParameterValue` "/Game/TRN_Snow/TRN_Materials/MPC_Capture.MPC_Capture" "CaptureSize" (`SceneCaptureComponent2D.OrthoWidth` (`self.SceneCapture`)))
  (bind _returnvalue (`KismetMaterialLibrary.CreateDynamicMaterialInstance` "/Game/TRN_Snow/TRN_Materials/M_DrawToPersistent.M_DrawToPersistent"))
  (set `self.DrawMaterial` _returnvalue)
  (`KismetRenderingLibrary.ClearRenderTarget2D` "/Game/TRN_Snow/TRN_RenderTargets/RT_Capture.RT_Capture")
  (`KismetRenderingLibrary.ClearRenderTarget2D` "/Game/TRN_Snow/TRN_RenderTargets/RT_Persistent.RT_Persistent"))

(event `self.ReceiveTick`
  (params (DeltaSeconds :type "Float (single-precision)"))
  (`self.DrawToPersistent`))

(fn `DrawToPersistent`
  (`KismetRenderingLibrary.DrawMaterialToRenderTarget` "/Game/TRN_Snow/TRN_RenderTargets/RT_Persistent.RT_Persistent" (`self.DrawMaterial`)))

(fn `UserConstructionScript`)