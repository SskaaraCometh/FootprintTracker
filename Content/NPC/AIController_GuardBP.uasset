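; AI controller for guard NPCs that turns perception updates and patrol data into Blackboard values.
; Sensed Enemy-tagged actors set the enemy key, which clears when they are lost.
; For other sensed actors, a Footprint tag sets the Footprint key and any other actor clears it.
; Find Route writes the guard pawn's first patrol point to the Waypoint key.
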(event `self.ReceiveBeginPlay`
  (set `self.BlackboardComp` (`self.BBComp`)))

(event `self.PerceptionComp.OnTargetPerceptionUpdated`
  (params (Actor :type "Actor Object Reference") (Stimulus :type "AIStimulus Structure"))
  (bind (_age _expirationage _strength _stimuluslocation _receiverlocation _tag _bsuccessfullysensed) (break `AIStimulus` Stimulus))
  (bind _blackboardcomp (`self.BlackboardComp`))
  (bind _enemykey (`self.EnemyKey`))
  (bind _blackboardcomp_2 (`self.BlackboardComp`))
  (bind _footprint (`self.Footprint`))
  (if (`self.ActorHasTag` Actor "Enemy")
    (if _bsuccessfullysensed
      (`BlackboardComponent.SetValueAsObject` _blackboardcomp_2 _enemykey Actor)
      (else
        (`BlackboardComponent.ClearValue` _blackboardcomp_2 _enemykey)))
    (elif _bsuccessfullysensed
      (if (`self.ActorHasTag` Actor "Footprint")
        (`BlackboardComponent.SetValueAsObject` _blackboardcomp _footprint Actor)
        (else
          (`BlackboardComponent.ClearValue` _blackboardcomp _footprint))))))

(fn `Find Route`
  (params (BlackboardComp :type "BlackboardComponent Object Reference"))
  (bind _asnpc_guard (cast `/Game/NPC/NPC_Guard` (`self.K2_GetPawn`)))
  (`BlackboardComponent.SetValueAsObject` BlackboardComp "Waypoint" (`|GetArrayItem` (`/Game/NPC/NPC_Guard.PatrolPoints` _asnpc_guard))))

(fn `UserConstructionScript`)